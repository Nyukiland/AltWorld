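; Shader-matching puzzle ball: the player edits its moving-noise material with keyboard keys to match a randomized OtherSphere.
; Per-parameter components handle change, randomization, comparison and syncing on a dynamic material instance; X cycles the edited color.
; Tick compares parameters unlocked by ShaderLevel, colors first, and copies the rest to OtherSphere.
; A full match raises the level and re-randomizes OtherSphere with more active parameters.
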(event `self.ReceiveBeginPlay`
  (bind _rotation (`self.Rotation`))
  (bind _amplitude (`self.Amplitude`))
  (bind _amplitude2 (`self.Amplitude2`))
  (bind _frequencex2 (`self.FrequenceX2`))
  (bind _frequencey (`self.FrequenceY`))
  (bind _frequencey2 (`self.FrequenceY2`))
  (bind _linewidth (`self.LineWidth`))
  (bind _linewidth2 (`self.LineWidth2`))
  (bind _linefade (`self.LineFade`))
  (bind _linefade2 (`self.LineFade2`))
  (bind _rotation2 (`self.Rotation2`))
  (bind _frequencex (`self.FrequenceX`))
  (bind _returnvalue (`PrimitiveComponent.CreateDynamicMaterialInstance` (`self.SphereTooDense`) 0 "/Game/Materials/MA_MovingNoiseTest.MA_MovingNoiseTest" "None"))
  (set `self.Material` _returnvalue)
  (`KismetArrayLibrary.Array_Clear` (`self.AllComponents`))
  (`/Game/BP_ParameterComponent.Init` _rotation (`self.Material`) "Rotation" 0.1 (0.0 0.0 0.0) (0.0 1.0) 0.1 false)
  (`KismetArrayLibrary.Array_Add` (`self.AllComponents`) _rotation)
  (`/Game/BP_ParameterComponent.Init` _rotation2 (`self.Material`) "Rotation2" 0.1 (0.0 0.0 0.0) (0.0 1.0) 0.1 false)
  (`KismetArrayLibrary.Array_Add` (`self.AllComponents`) _rotation2)
  (`/Game/BP_ParameterComponent.Init` _amplitude (`self.Material`) "Amplitude" 1.0 (0.0 0.0 0.0) (1.0 10.0) 1.0 false)
  (`KismetArrayLibrary.Array_Add` (`self.AllComponents`) _amplitude)
  (`/Game/BP_ParameterComponent.Init` _amplitude2 (`self.Material`) "Amplitude2" 1.0 (0.0 0.0 0.0) (1.0 10.0) 1.0 false)
  (`KismetArrayLibrary.Array_Add` (`self.AllComponents`) _amplitude2)
  (`/Game/BP_ParameterComponent.Init` _frequencex (`self.Material`) "FrequencyX" 1.0 (0.0 0.0 0.0) (0.1 10.0) 1.0 false)
  (`KismetArrayLibrary.Array_Add` (`self.AllComponents`) _frequencex)
  (`/Game/BP_ParameterComponent.Init` _frequencex2 (`self.Material`) "FrequencyX2" 1.0 (0.0 0.0 0.0) (0.1 10.0) 1.0 false)
  (`KismetArrayLibrary.Array_Add` (`self.AllComponents`) _frequencex2)
  (`/Game/BP_ParameterComponent.Init` _frequencey (`self.Material`) "FrequencyY" 1.0 (0.0 0.0 0.0) (0.1 10.0) 1.0 false)
  (`KismetArrayLibrary.Array_Add` (`self.AllComponents`) _frequencey)
  (`/Game/BP_ParameterComponent.Init` _frequencey2 (`self.Material`) "FrequencyY2" 1.0 (0.0 0.0 0.0) (0.1 10.0) 1.0 false)
  (`KismetArrayLibrary.Array_Add` (`self.AllComponents`) _frequencey2)
  (`/Game/BP_ParameterComponent.Init` _linewidth (`self.Material`) "LineThickness" 1.0 (1.0 0.0 0.0) (0.2 10.0) 1.0 false)
  (`KismetArrayLibrary.Array_Add` (`self.AllComponents`) _linewidth)
  (`/Game/BP_ParameterComponent.Init` _linewidth2 (`self.Material`) "LineThickness2" 1.0 (1.0 0.0 0.0) (0.2 10.0) 1.0 false)
  (`KismetArrayLibrary.Array_Add` (`self.AllComponents`) _linewidth2)
  (`/Game/BP_ParameterComponent.Init` _linefade (`self.Material`) "LineThickness" 0.1 (0.0 1.0 0.0) (0.1 1.0) 0.1 false)
  (`KismetArrayLibrary.Array_Add` (`self.AllComponents`) _linefade)
  (`/Game/BP_ParameterComponent.Init` _linefade2 (`self.Material`) "LineThickness2" 0.1 (0.0 1.0 0.0) (0.1 1.0) 0.1 false)
  (`KismetArrayLibrary.Array_Add` (`self.AllComponents`) _linefade2)
  (`/Game/BP_ParameterComponent.Init` (`self.RedChannel`) (`self.Material`) " " 0.1 (1.0 0.0 0.0) (0.0 1.0) 1.0 false)
  (`/Game/BP_ParameterComponent.Init` (`self.BlueChannel`) (`self.Material`) " " 0.1 (0.0 0.0 1.0) (0.0 1.0) 0.1 false)
  (`/Game/BP_ParameterComponent.Init` (`self.GreenChannel`) (`self.Material`) " " 0.1 (0.0 1.0 0.0) (0.0 1.0) 0.1 false)
  (`/Game/BP_ParameterComponent.Init` (`self.Height`) (`self.Material`) "UpHeight" 50.0 (0.0 0.0 0.0) (-100.0 200.0) 0.1 false)
  (set `self.CurColor` (`|GetArrayItem` (`self.ColorParamName`)))
  ; Ignores code for the small sphere that has no "PlayerSphere" reference
  (`/Engine/EditorBlueprintResources/StandardMacros.IsValid` (`self.OtherSphere`)
    (:`Is Valid`
      (`self.RandomizeValues` (`self.OtherSphere`) 0))))

(event `Key|Q`
  (params (Key :type "Key Structure"))
  (:`Pressed`
    (`/Game/BP_ParameterComponent.CallChange` (`self.Amplitude`) "None"))
  (:`Released`
    (`/Game/BP_ParameterComponent.CallChange` (`self.Amplitude`) "None")))

(event `Key|W`
  (params (Key :type "Key Structure"))
  (:`Pressed`
    (`/Game/BP_ParameterComponent.CallChange` (`self.FrequenceX`) "None"))
  (:`Released`
    (`/Game/BP_ParameterComponent.CallChange` (`self.FrequenceX`) "None")))

(event `Key|E`
  (params (Key :type "Key Structure"))
  (:`Pressed`
    (`/Game/BP_ParameterComponent.CallChange` (`self.FrequenceY`) "None"))
  (:`Released`
    (`/Game/BP_ParameterComponent.CallChange` (`self.FrequenceY`) "None")))

(event `Key|R`
  (params (Key :type "Key Structure"))
  (:`Pressed`
    (`/Game/BP_ParameterComponent.CallChange` (`self.Rotation`) "None"))
  (:`Released`
    (`/Game/BP_ParameterComponent.CallChange` (`self.Rotation`) "None")))

(event `Key|T`
  (params (Key :type "Key Structure"))
  (:`Pressed`
    (`/Game/BP_ParameterComponent.CallChange` (`self.LineWidth`) "None"))
  (:`Released`
    (`/Game/BP_ParameterComponent.CallChange` (`self.LineWidth`) "None")))

(event `Key|Y`
  (params (Key :type "Key Structure"))
  (:`Pressed`
    (`/Game/BP_ParameterComponent.CallChange` (`self.LineFade`) "None"))
  (:`Released`
    (`/Game/BP_ParameterComponent.CallChange` (`self.LineFade`) "None")))

(event `Key|Z`
  (params (Key :type "Key Structure"))
  (:`Pressed`
    (`/Game/BP_ParameterComponent.CallChange` (`self.Height`) "None"))
  (:`Released`
    (`/Game/BP_ParameterComponent.CallChange` (`self.Height`) "None")))

(event `Key|C`
  (params (Key :type "Key Structure"))
  (:`Pressed`
    (`/Game/BP_ParameterComponent.CallChange` (`self.RedChannel`) (`self.CurColor`)))
  (:`Released`
    (`/Game/BP_ParameterComponent.CallChange` (`self.RedChannel`) "None")))

(event `Key|B`
  (params (Key :type "Key Structure"))
  (:`Pressed`
    (`/Game/BP_ParameterComponent.CallChange` (`self.BlueChannel`) (`self.CurColor`)))
  (:`Released`
    (`/Game/BP_ParameterComponent.CallChange` (`self.BlueChannel`) "None")))

(event `Key|A`
  (params (Key :type "Key Structure"))
  (:`Pressed`
    (`/Game/BP_ParameterComponent.CallChange` (`self.Amplitude2`) "None"))
  (:`Released`
    (`/Game/BP_ParameterComponent.CallChange` (`self.Amplitude2`) "None")))

(event `Key|S`
  (params (Key :type "Key Structure"))
  (:`Pressed`
    (`/Game/BP_ParameterComponent.CallChange` (`self.FrequenceX2`) "None"))
  (:`Released`
    (`/Game/BP_ParameterComponent.CallChange` (`self.FrequenceX2`) "None")))

(event `Key|D`
  (params (Key :type "Key Structure"))
  (:`Pressed`
    (`/Game/BP_ParameterComponent.CallChange` (`self.FrequenceY2`) "None"))
  (:`Released`
    (`/Game/BP_ParameterComponent.CallChange` (`self.FrequenceY2`) "None")))

(event `Key|F`
  (params (Key :type "Key Structure"))
  (:`Pressed`
    (`/Game/BP_ParameterComponent.CallChange` (`self.Rotation2`) "None"))
  (:`Released`
    (`/Game/BP_ParameterComponent.CallChange` (`self.Rotation2`) "None")))

(event `Key|G`
  (params (Key :type "Key Structure"))
  (:`Pressed`
    (`/Game/BP_ParameterComponent.CallChange` (`self.LineWidth2`) "None"))
  (:`Released`
    (`/Game/BP_ParameterComponent.CallChange` (`self.LineWidth2`) "None")))

(event `Key|H`
  (params (Key :type "Key Structure"))
  (:`Pressed`
    (`/Game/BP_ParameterComponent.CallChange` (`self.LineFade2`) "None"))
  (:`Released`
    (`/Game/BP_ParameterComponent.CallChange` (`self.LineFade2`) "None")))

(event `Key|X`
  (params (Key :type "Key Structure"))
  (bind _colorparamname (`self.ColorParamName`))
  (:`Pressed`
    (bind _result (`/Engine/EditorBlueprintResources/StandardMacros.IncrementInt` (`self.IndexColor`))
      (:`  `
        (if (>= _result (`KismetArrayLibrary.Array_Length` _colorparamname))
          (set `self.IndexColor` 0))
        (set `self.CurColor` (`|GetArrayItem` _colorparamname (`self.IndexColor`)))))))

(event `Key|V`
  (params (Key :type "Key Structure"))
  (:`Pressed`
    (`/Game/BP_ParameterComponent.CallChange` (`self.GreenChannel`) (`self.CurColor`)))
  (:`Released`
    (`/Game/BP_ParameterComponent.CallChange` (`self.GreenChannel`) "None")))

(event `self.ReceiveTick`
  (params (DeltaSeconds :type "Float (single-precision)"))
  (`/Engine/EditorBlueprintResources/StandardMacros.IsValid` (`self.OtherSphere`)
    (:`Is Valid`
      (bind _issimilar (`self.CompareValues`))
      (if _issimilar
        (bind _output_get (set `self.ShaderLevel` (`KismetMathLibrary.Clamp` (+ (`self.ShaderLevel`) 1) 0 (`self.GetMaxParameter`))))
        (`self.RandomizeValues` (`self.OtherSphere`) _output_get)
        (`KismetSystemLibrary.PrintString` (`KismetStringLibrary.Concat_StrStr` "=========================================================" "GOING TO LEVEL " (`KismetStringLibrary.Conv_IntToString` _output_get) "========================================================="))))))

(fn `CompareValues`
  (returns (IsSimilar :type Boolean))
  (locals (TrueValues :type Integer) (CheckedValue :type Integer))
  (`/Engine/EditorBlueprintResources/StandardMacros.IsValid` (`self.OtherSphere`)
    (:`Is Valid`
      (for (_array_element _array_index) (`self.ColorParamName`)
        (if (<= _array_index (`self.ShaderLevel`))
          ; Compare
          (bind _returnvalue (`MaterialInstanceDynamic.K2_GetVectorParameterValue` (`/Game/BP_Ball.Material` (`self.OtherSphere`)) _array_element))
          (bind _result (`/Game/BP_ParameterComponent.CallCompare` (`self.RedChannel`) _array_element 0.0 _returnvalue))
          (`/Engine/EditorBlueprintResources/StandardMacros.IncrementInt` (`local.CheckedValue`)
            (:`  `
              (if _result
                (`/Engine/EditorBlueprintResources/StandardMacros.IncrementInt` (`local.TrueValues`)))))
          (else
            (bind _returnvalue_2 (`MaterialInstanceDynamic.K2_GetVectorParameterValue` (`self.Material`) _array_element))
            (`/Game/BP_ParameterComponent.SyncValue` (`/Game/BP_Ball.RedChannel` (`self.OtherSphere`)) _array_element _returnvalue_2 0.0))))
      (for (_array_element_2 _array_index_2) (`self.AllComponents`)
        (if (<= _array_index_2 (- (`self.ShaderLevel`) (`KismetArrayLibrary.Array_Length` (`self.ColorParamName`))))
          (bind _output (`|GetArrayItem` (`/Game/BP_Ball.AllComponents` (`self.OtherSphere`)) _array_index_2))
          (bind _results (`/Game/BP_ParameterComponent.GetVectorValue` _output))
          (bind _result_2 (`/Game/BP_ParameterComponent.GetFloatValue` _output))
          (bind _result_3 (`/Game/BP_ParameterComponent.CallCompare` _array_element_2 (`/Game/BP_ParameterComponent.Parameter Name` _array_element_2) _result_2 _results))
          (`/Engine/EditorBlueprintResources/StandardMacros.IncrementInt` (`local.CheckedValue`)
            (:`  `
              (if _result_3
                (`/Engine/EditorBlueprintResources/StandardMacros.IncrementInt` (`local.TrueValues`)))))
          (else
            (bind _results_2 (`/Game/BP_ParameterComponent.GetVectorValue` _array_element_2))
            (bind _result_4 (`/Game/BP_ParameterComponent.GetFloatValue` _array_element_2))
            (bind _output_2 (`|GetArrayItem` (`/Game/BP_Ball.AllComponents` (`self.OtherSphere`)) _array_index_2))
            (`/Game/BP_ParameterComponent.SyncValue` _output_2 (`/Game/BP_ParameterComponent.Parameter Name` _output_2) _results_2 _result_4))))
      (`KismetSystemLibrary.PrintString` (`KismetStringLibrary.Concat_StrStr` (`KismetStringLibrary.Conv_IntToString` (`local.TrueValues`)) "/" (`KismetStringLibrary.Conv_IntToString` (`local.CheckedValue`)) " are similar"))
      (return (== (`local.CheckedValue`) (`local.TrueValues`))))
    (:`Is Not Valid`
      (return false))))

(fn `RandomizeValues`
  (params (ShaderLevel :type Integer))
  (bind _returnvalue (`KismetArrayLibrary.Array_Length` (`self.ColorParamName`)))
  (set `self.ShaderLevel` ShaderLevel)
  (for (_array_element _array_index) (`self.ColorParamName`)
    (if (<= _array_index (`self.ShaderLevel`))
      (`/Game/BP_ParameterComponent.CallRandomize` (`self.RedChannel`) _array_element)))
  (if (>= (`self.ShaderLevel`) _returnvalue)
    (for (_array_element_2 _array_index_2) (`self.AllComponents`)
      (if (<= _array_index_2 (- (`self.ShaderLevel`) _returnvalue))
        (`/Game/BP_ParameterComponent.CallRandomize` _array_element_2 (`/Game/BP_ParameterComponent.Parameter Name` _array_element_2))))))

(fn `UserConstructionScript`)