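; Component that drives one scalar material parameter through click-based steps, apparently for a sphere-matching puzzle.
; Init binds the material, parameter, step, clamp range and tolerance; clicks step the target value, bouncing between limits when no direction is given.
; Tick lerps the material parameter toward that target for a smooth transition.
; Helpers randomize the target on step increments and compare it to another value, returning a tolerance match and closeness percentage.
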(event `Init`
  (params (Material :type "MaterialInstanceDynamic Object Reference") (ParameterName :type Name) (ValueChange :type "Float (double-precision)") (ClampValue :type "Vector2D Structure") (Tolerance :type "Float (double-precision)"))
  (set `self.Material` Material)
  (set `self.Parameter Name` ParameterName)
  (set `self.Value Change` ValueChange)
  (set `self.ClampValue` ClampValue)
  (set `self.Tolerance` Tolerance)
  (bind _returnvalue (`MaterialInstanceDynamic.K2_GetScalarParameterValue` (`self.Material`) (`self.Parameter Name`)))
  (set `self.AimedValueFloat` _returnvalue))

(event `self.ReceiveTick`
  (params (DeltaSeconds :type "Float (single-precision)"))
  (set `self.Delta Seconds` DeltaSeconds)
  (`self.ChangeFloatToAimedValue`))

(fn `ChangeFloatClick`
  (params (value :type Integer))
  (locals (Check :type Boolean :default false))
  (bind (_x _y) (`KismetMathLibrary.BreakVector2D` (`self.ClampValue`)))
  (bind (_x_2 _y_2) (`KismetMathLibrary.BreakVector2D` (`self.ClampValue`)))
  (bind _returnvalue (`KismetMathLibrary.FClamp` (+ (`self.AimedValueFloat`) (* (`self.Value Change`) (`self.GoUp`))) _x_2 _y_2))
  (if (!= value 0)
    (set `self.AimedValueFloat` (`KismetMathLibrary.FClamp` (+ (`self.AimedValueFloat`) (* (`self.Value Change`) value)) _x _y))
    (else
      (bind _output_get (set `local.Check` (or (== _returnvalue _x_2) (== _returnvalue _y_2))))
      (set `self.AimedValueFloat` _returnvalue)
      (if _output_get
        (set `self.GoUp` (* (`self.GoUp`) -1))))))

(fn `ChangeFloatToAimedValue`
  (locals (GoUpRed :type Integer) (GoUpGreen :type Integer) (GoUpBlue :type Integer) (CurrentParameterValue :type "LinearColor Structure") (RedClampValue :type "Vector2D Structure") (GreenClampValue :type "Vector2D Structure") (BlueClampValue :type "Vector2D Structure"))
  (bind _returnvalue (`MaterialInstanceDynamic.K2_GetScalarParameterValue` (`self.Material`) (`self.Parameter Name`)))
  (`MaterialInstanceDynamic.SetScalarParameterValue` (`self.Material`) (`self.Parameter Name`) (`KismetMathLibrary.Lerp` _returnvalue (`self.AimedValueFloat`) (* (`self.Delta Seconds`) (`self.LerpSpeed`)))))

(fn `CompareFloat`
  (params (OtherSphereValue :type "Float (double-precision)"))
  (returns (Result :type Boolean) (Percentage :type "Float (double-precision)"))
  (locals (ValueToCompare :type "Float (double-precision)") (RangeValue :type "Float (double-precision)") (Parameter :type Name))
  (bind _aimedvaluefloat (`self.AimedValueFloat`))
  (bind _valuetocompare (`local.ValueToCompare`))
  (bind (_clampvalue_x _clampvalue_y) (`KismetMathLibrary.BreakVector2D` (`self.ClampValue`)))
  (set `local.ValueToCompare` OtherSphereValue)
  (set `local.RangeValue` (`KismetMathLibrary.Abs` (- _clampvalue_x _clampvalue_y)))
  (`KismetSystemLibrary.PrintString` (`KismetStringLibrary.Concat_StrStr` (`KismetStringLibrary.Conv_DoubleToString` _aimedvaluefloat) " / " (`KismetStringLibrary.Conv_DoubleToString` _valuetocompare)))
  (return (`KismetMathLibrary.NearlyEqual_FloatFloat` _aimedvaluefloat _valuetocompare (`self.Tolerance`)) (- 1.0 (/ (`KismetMathLibrary.Abs` (- _aimedvaluefloat (`local.ValueToCompare`))) (`local.RangeValue`)))))

(fn `DetermineMaximumDifference`
  (params (Value :type "Float (double-precision)"))
  (returns (Difference :type "Float (double-precision)"))
  (locals (HalfRangeValue :type "Float (double-precision)") (VectorToAnalyze :type "LinearColor Structure") (MaxClampValue :type "Float (double-precision)") (DifferenceToReturn :type "Float (double-precision)") (MinClampValue :type "Float (double-precision)") (ValueToAnalyze :type "Float (double-precision)"))
  (bind _valuetoanalyze (`local.ValueToAnalyze`))
  (bind (_clampvalue_x _clampvalue_y) (`KismetMathLibrary.BreakVector2D` (`self.ClampValue`)))
  (set `local.ValueToAnalyze` Value)
  (set `local.MinClampValue` _clampvalue_x)
  (set `local.MaxClampValue` _clampvalue_y)
  (set `local.HalfRangeValue` (/ (`KismetMathLibrary.Abs` (- _clampvalue_x 0.0)) 2.0))
  (if (>= (`local.HalfRangeValue`) _valuetoanalyze)
    ; if value to find is closer to min clamp value
    (set `local.DifferenceToReturn` (- (`local.MaxClampValue`) _valuetoanalyze))
    (else
      ; if value to find is closer to max clamp value
      (set `local.DifferenceToReturn` (- _valuetoanalyze (`local.MinClampValue`)))))
  (return (`local.DifferenceToReturn`)))

(fn `GetRandomFloat`
  (params (currentValue :type "Float (double-precision)"))
  (returns (returnValue :type "Float (double-precision)"))
  (bind (_clampvalue_x _clampvalue_y) (`KismetMathLibrary.BreakVector2D` (`self.ClampValue`)))
  (bind _clampvalue_x_2 (`KismetMathLibrary.BreakVector2D` (`self.ClampValue`)))
  (bind (_clampvalue_x_3 _clampvalue_y_2) (`KismetMathLibrary.BreakVector2D` (`self.ClampValue`)))
  (bind (_clampvalue_x_4 _clampvalue_y_3) (`KismetMathLibrary.BreakVector2D` (`self.ClampValue`)))
  (bind _clampvalue_x_5 (`KismetMathLibrary.BreakVector2D` (`self.ClampValue`)))
  (bind _returnvalue (`KismetMathLibrary.FTrunc` (/ (- _clampvalue_y_3 _clampvalue_x_4) (`self.Value Change`))))
  (if (< (- currentValue _clampvalue_x) (- _clampvalue_y _clampvalue_x))
    (return (+ (* (`KismetMathLibrary.RandomIntegerInRange` (/ _returnvalue 2) _returnvalue) (`self.Value Change`)) _clampvalue_x_2))
    (else
      (return (+ (* (`KismetMathLibrary.RandomIntegerInRange` 0 (/ (`KismetMathLibrary.FTrunc` (/ (- _clampvalue_y_2 _clampvalue_x_3) (`self.Value Change`))) 2)) (`self.Value Change`)) _clampvalue_x_5)))))

(fn `RandomizeFloat`
  (set `self.AimedValueFloat` (`self.GetRandomFloat` (`self.AimedValueFloat`))))