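; Test character Blueprint that drives a post-process effect, apparently a Julia fractal, from the keyboard.
; Each key press reads a parameter from the MPC_PostPro Material Parameter Collection and writes it back shifted by a fixed step.
; Q/E adjust the Julia value, Shift/Ctrl adjust Zoom, and WASD pan the Offset vector through its R and G channels.
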(event `Key|Q`
  (params (Key :type "Key Structure"))
  (:`Pressed`
    (bind _returnvalue (`KismetMaterialLibrary.GetScalarParameterValue` "/Game/Materials/MPC_PostPro.MPC_PostPro" "Julia"))
    (`KismetMaterialLibrary.SetScalarParameterValue` "/Game/Materials/MPC_PostPro.MPC_PostPro" "Julia" (+ _returnvalue -0.1))))

(event `Key|E`
  (params (Key :type "Key Structure"))
  (:`Pressed`
    (bind _returnvalue (`KismetMaterialLibrary.GetScalarParameterValue` "/Game/Materials/MPC_PostPro.MPC_PostPro" "Julia"))
    (`KismetMaterialLibrary.SetScalarParameterValue` "/Game/Materials/MPC_PostPro.MPC_PostPro" "Julia" (+ _returnvalue 0.1))))

(event `Key|LeftShift`
  (params (Key :type "Key Structure"))
  (:`Pressed`
    (bind _returnvalue (`KismetMaterialLibrary.GetScalarParameterValue` "/Game/Materials/MPC_PostPro.MPC_PostPro" "Zoom"))
    (`KismetMaterialLibrary.SetScalarParameterValue` "/Game/Materials/MPC_PostPro.MPC_PostPro" "Zoom" (+ _returnvalue -0.1))))

(event `Key|LeftControl`
  (params (Key :type "Key Structure"))
  (:`Pressed`
    (bind _returnvalue (`KismetMaterialLibrary.GetScalarParameterValue` "/Game/Materials/MPC_PostPro.MPC_PostPro" "Zoom"))
    (`KismetMaterialLibrary.SetScalarParameterValue` "/Game/Materials/MPC_PostPro.MPC_PostPro" "Zoom" (+ _returnvalue 0.1))))

(event `Key|W`
  (params (Key :type "Key Structure"))
  (:`Pressed`
    (bind _returnvalue (`KismetMaterialLibrary.GetVectorParameterValue` "/Game/Materials/MPC_PostPro.MPC_PostPro" "Offset"))
    (bind (_r _g _b _a) (`KismetMathLibrary.BreakColor` _returnvalue))
    (`KismetMaterialLibrary.SetVectorParameterValue` "/Game/Materials/MPC_PostPro.MPC_PostPro" "Offset" (`KismetMathLibrary.MakeColor` _r (+ _g 0.1) _b _a))))

(event `Key|S`
  (params (Key :type "Key Structure"))
  (:`Pressed`
    (bind _returnvalue (`KismetMaterialLibrary.GetVectorParameterValue` "/Game/Materials/MPC_PostPro.MPC_PostPro" "Offset"))
    (bind (_r _g _b _a) (`KismetMathLibrary.BreakColor` _returnvalue))
    (`KismetMaterialLibrary.SetVectorParameterValue` "/Game/Materials/MPC_PostPro.MPC_PostPro" "Offset" (`KismetMathLibrary.MakeColor` _r (+ _g -0.1) _b _a))))

(event `Key|A`
  (params (Key :type "Key Structure"))
  (:`Pressed`
    (bind _returnvalue (`KismetMaterialLibrary.GetVectorParameterValue` "/Game/Materials/MPC_PostPro.MPC_PostPro" "Offset"))
    (bind (_r _g _b _a) (`KismetMathLibrary.BreakColor` _returnvalue))
    (`KismetMaterialLibrary.SetVectorParameterValue` "/Game/Materials/MPC_PostPro.MPC_PostPro" "Offset" (`KismetMathLibrary.MakeColor` (+ _r 0.1) _g _b _a))))

(event `Key|D`
  (params (Key :type "Key Structure"))
  (:`Pressed`
    (bind _returnvalue (`KismetMaterialLibrary.GetVectorParameterValue` "/Game/Materials/MPC_PostPro.MPC_PostPro" "Offset"))
    (bind (_r _g _b _a) (`KismetMathLibrary.BreakColor` _returnvalue))
    (`KismetMaterialLibrary.SetVectorParameterValue` "/Game/Materials/MPC_PostPro.MPC_PostPro" "Offset" (`KismetMathLibrary.MakeColor` (+ _r -0.1) _g _b _a))))

(fn `UserConstructionScript`)