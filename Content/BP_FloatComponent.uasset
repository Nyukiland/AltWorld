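; BP_FloatComponent smoothly drives one named scalar parameter on a material toward a target float.
; Init stores the material, parameter name and clamp value, then seeds the target from the parameter's current value.
; Each Tick reads the live value and lerps it toward the target by delta time times LerpSpeed, giving an eased approach.
; The clamp value is stored but unused in these graphs.
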(event `Init`
  (params (Material :type "MaterialInstanceDynamic Object Reference") (ParameterName :type Name) (ClampValue :type "Vector2D Structure"))
  (set `self.Material` Material)
  (set `self.Parameter Name` ParameterName)
  (set `self.Clamp Value` ClampValue)
  (bind _returnvalue (`MaterialInstanceDynamic.K2_GetScalarParameterValue` (`self.Material`) (`self.Parameter Name`)))
  (set `self.AimedValueFloat` _returnvalue))

(event `self.ReceiveTick`
  (params (DeltaSeconds :type "Float (single-precision)"))
  (set `self.Delta Seconds` DeltaSeconds)
  (`self.ChangeFloatToAimedValue`))

(fn `ChangeFloatToAimedValue`
  (locals (GoUpRed :type Integer) (GoUpGreen :type Integer) (GoUpBlue :type Integer) (CurrentParameterValue :type "LinearColor Structure") (RedClampValue :type "Vector2D Structure") (GreenClampValue :type "Vector2D Structure") (BlueClampValue :type "Vector2D Structure"))
  (bind _returnvalue (`MaterialInstanceDynamic.K2_GetScalarParameterValue` (`self.Material`) (`self.Parameter Name`)))
  (`MaterialInstanceDynamic.SetScalarParameterValue` (`self.Material`) (`self.Parameter Name`) (`KismetMathLibrary.Lerp` _returnvalue (`self.AimedValueFloat`) (* (`self.Delta Seconds`) (`self.LerpSpeed`)))))