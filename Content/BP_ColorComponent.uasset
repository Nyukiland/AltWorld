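; Color component for what appears to be a sphere color-matching game, driving a vector parameter on a material supplied through Init.
; Per-channel click functions step the target color within clamp bounds, reversing direction upon reaching 0 or 1, while RandomizeVector picks stepped random values.
; Tick lerps the material's current color toward that target.
; CompareVector checks the target against another sphere's color, returning a tolerance-based match and a similarity percentage.
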(event `Init`
  (params (Material :type "MaterialInstanceDynamic Object Reference") (ParameterName :type Name) (ValueChange :type "Float (double-precision)") (ClampValue :type "Vector2D Structure") (Tolerance :type "Float (double-precision)"))
  (set `self.Material` Material)
  (set `self.Parameter Name` ParameterName)
  (set `self.Value Change` ValueChange)
  (set `self.ClampValue` ClampValue)
  (set `self.Tolerance` Tolerance)
  (bind _returnvalue (`MaterialInstanceDynamic.K2_GetVectorParameterValue` (`self.Material`) (`self.Parameter Name`)))
  (set `self.AimedValueVector` _returnvalue))

(event `self.ReceiveTick`
  (params (DeltaSeconds :type "Float (single-precision)"))
  (set `self.Delta Seconds` DeltaSeconds)
  (`self.ChangeVectorToAimedValues`))

(fn `ChangeBlueClick`
  (locals (CheckValue :type Boolean :default false))
  (bind (_r _g _b) (break `LinearColor` (`self.AimedValueVector`)))
  (bind (_x _y) (`KismetMathLibrary.BreakVector2D` (`self.ClampValue`)))
  (bind _returnvalue (`KismetMathLibrary.FClamp` (+ _b (* (`self.Value Change`) (`self.BlueGoUp`))) _x _y))
  (set `local.CheckValue` (or (== _returnvalue 0.0) (== _returnvalue 1.0)))
  (set `self.AimedValueVector` (`KismetMathLibrary.MakeColor` _r _g _returnvalue))
  (if (`local.CheckValue`)
    (set `self.BlueGoUp` (* (`self.BlueGoUp`) -1))))

(fn `ChangeGreenClick`
  (locals (CheckValue :type Boolean :default false))
  (bind (_r _g _b) (break `LinearColor` (`self.AimedValueVector`)))
  (bind (_x _y) (`KismetMathLibrary.BreakVector2D` (`self.ClampValue`)))
  (bind _returnvalue (`KismetMathLibrary.FClamp` (+ _g (* (`self.Value Change`) (`self.GreenGoUp`))) _x _y))
  (set `local.CheckValue` (or (== _returnvalue 0.0) (== _returnvalue 1.0)))
  (set `self.AimedValueVector` (`KismetMathLibrary.MakeColor` _r _returnvalue _b))
  (if (`local.CheckValue`)
    (set `self.GreenGoUp` (* (`self.GreenGoUp`) -1))))

(fn `ChangeRedClick`
  (locals (CheckValue :type Boolean :default false))
  (bind (_r _g _b) (break `LinearColor` (`self.AimedValueVector`)))
  (bind (_x _y) (`KismetMathLibrary.BreakVector2D` (`self.ClampValue`)))
  (bind _returnvalue (`KismetMathLibrary.FClamp` (+ _r (* (`self.Value Change`) (`self.RedGoUp`))) _x _y))
  (set `local.CheckValue` (or (== _returnvalue 0.0) (== _returnvalue 1.0)))
  (set `self.AimedValueVector` (`KismetMathLibrary.MakeColor` _returnvalue _g _b))
  (if (`local.CheckValue`)
    (set `self.RedGoUp` (* (`self.RedGoUp`) -1))))

(fn `ChangeVectorToAimedValues`
  (locals (GoUpRed :type Integer) (GoUpGreen :type Integer) (GoUpBlue :type Integer) (CurrentParameterValue :type "LinearColor Structure") (RedClampValue :type "Vector2D Structure") (GreenClampValue :type "Vector2D Structure") (BlueClampValue :type "Vector2D Structure"))
  (bind _returnvalue (`MaterialInstanceDynamic.K2_GetVectorParameterValue` (`self.Material`) (`self.Parameter Name`)))
  (`MaterialInstanceDynamic.SetVectorParameterValue` (`self.Material`) (`self.Parameter Name`) (`KismetMathLibrary.LinearColorLerp` _returnvalue (`self.AimedValueVector`) (* (`self.Delta Seconds`) (`self.LerpSpeed`)))))

(fn `CompareVector`
  (params (OtherSphereValue :type "LinearColor Structure"))
  (returns (Result :type Boolean) (Percentage :type "Float (double-precision)"))
  (locals (MaximumVectorDifference :type "Float (double-precision)") (PercentageToReturn :type "Float (double-precision)") (ValueToCompare :type "LinearColor Structure") (RangeValue :type "Float (double-precision)"))
  (bind _aimedvaluevector (`self.AimedValueVector`))
  (bind (_clampvalue_x _clampvalue_y) (`KismetMathLibrary.BreakVector2D` (`self.ClampValue`)))
  (bind (_returnvalue_r _returnvalue_g _returnvalue_b) (break `LinearColor` (- _aimedvaluevector (`local.ValueToCompare`))))
  (bind _returnvalue (- 1.0 (/ (+ (`KismetMathLibrary.Abs` _returnvalue_r) (`KismetMathLibrary.Abs` _returnvalue_g) (`KismetMathLibrary.Abs` _returnvalue_b)) (* 3.0 (`local.RangeValue`)))))
  (set `local.ValueToCompare` OtherSphereValue)
  (set `local.RangeValue` (`KismetMathLibrary.Abs` (- _clampvalue_x _clampvalue_y)))
  (set `local.PercentageToReturn` _returnvalue)
  (return (`KismetMathLibrary.LinearColor_IsNearEqual` _aimedvaluevector (`local.ValueToCompare`) (`self.Tolerance`)) _returnvalue))

(fn `DetermineMaximumDifference`
  (params (Value :type "Float (double-precision)"))
  (returns (Difference :type "Float (double-precision)"))
  (locals (HalfRangeValue :type "Float (double-precision)") (VectorToAnalyze :type "LinearColor Structure") (MaxClampValue :type "Float (double-precision)") (DifferenceToReturn :type "Float (double-precision)") (MinClampValue :type "Float (double-precision)") (ValueToAnalyze :type "Float (double-precision)"))
  (bind _valuetoanalyze (`local.ValueToAnalyze`))
  (bind (_clampvalue_x _clampvalue_y) (`KismetMathLibrary.BreakVector2D` (`self.ClampValue`)))
  (set `local.ValueToAnalyze` Value)
  (set `local.MinClampValue` _clampvalue_x)
  (set `local.MaxClampValue` _clampvalue_y)
  (set `local.HalfRangeValue` (/ (`KismetMathLibrary.Abs` (- _clampvalue_x 0.0)) 2.0))
  (if (>= (`local.HalfRangeValue`) _valuetoanalyze)
    ; if value to find is closer to min clamp value
    (set `local.DifferenceToReturn` (- (`local.MaxClampValue`) _valuetoanalyze))
    (else
      ; if value to find is closer to max clamp value
      (set `local.DifferenceToReturn` (- _valuetoanalyze (`local.MinClampValue`)))))
  (return (`local.DifferenceToReturn`)))

(fn `GetRandomFloat`
  (params (currentValue :type "Float (double-precision)"))
  (returns (returnValue :type "Float (double-precision)"))
  (bind (_clampvalue_x _clampvalue_y) (`KismetMathLibrary.BreakVector2D` (`self.ClampValue`)))
  (bind _clampvalue_x_2 (`KismetMathLibrary.BreakVector2D` (`self.ClampValue`)))
  (bind (_clampvalue_x_3 _clampvalue_y_2) (`KismetMathLibrary.BreakVector2D` (`self.ClampValue`)))
  (bind (_clampvalue_x_4 _clampvalue_y_3) (`KismetMathLibrary.BreakVector2D` (`self.ClampValue`)))
  (bind _clampvalue_x_5 (`KismetMathLibrary.BreakVector2D` (`self.ClampValue`)))
  (bind _returnvalue (`KismetMathLibrary.FTrunc` (/ (- _clampvalue_y_3 _clampvalue_x_4) (`self.Value Change`))))
  (if (< (- currentValue _clampvalue_x) (- _clampvalue_y _clampvalue_x))
    (return (+ (* (`KismetMathLibrary.RandomIntegerInRange` (/ _returnvalue 2) _returnvalue) (`self.Value Change`)) _clampvalue_x_2))
    (else
      (return (+ (* (`KismetMathLibrary.RandomIntegerInRange` 0 (/ (`KismetMathLibrary.FTrunc` (/ (- _clampvalue_y_2 _clampvalue_x_3) (`self.Value Change`))) 2)) (`self.Value Change`)) _clampvalue_x_5)))))

(fn `RandomizeVector`
  (bind (_r _g _b) (break `LinearColor` (`self.AimedValueVector`)))
  (set `self.AimedValueVector` (`KismetMathLibrary.MakeColor` (`self.GetRandomFloat` _r) (`self.GetRandomFloat` _g) (`self.GetRandomFloat` _b))))