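; Sphere for a shader-matching puzzle, where key presses tune its noise material's amplitude, frequency, rotation and colors to match a linked OtherSphere.
; Per-parameter components drive a dynamic material instance, with one key cycling the edited color.
; Tick compares both spheres, reports scores to WB_Level and, on a full match, re-randomizes OtherSphere by ShaderLevel.
; P toggles a reversible explosion that raises height, shifts colors and hides the mesh at maximum height.
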(event `self.ReceiveBeginPlay`
  (bind _amplitude1 (`self.Amplitude1`))
  (bind _amplitude2 (`self.Amplitude2`))
  (bind _rotation (`self.Rotation`))
  (bind _frequencyx2 (`self.FrequencyX2`))
  (bind _frequencyy1 (`self.FrequencyY1`))
  (bind _frequencyy2 (`self.FrequencyY2`))
  (bind _frequencyx1 (`self.FrequencyX1`))
  (bind _returnvalue (`PrimitiveComponent.CreateDynamicMaterialInstance` (`self.SphereTooDense`) 0 "/Game/Materials/MA_MovingNoiseTest.MA_MovingNoiseTest" "None"))
  (set `self.Material` _returnvalue)
  (bind _returnvalue_2 (`|CreateWidget` "/Game/UI/WB_Level.WB_Level_C" (`GameplayStatics.GetPlayerController` 0)))
  (set `self.HudWidget` _returnvalue_2)
  (`UserWidget.AddToViewport` _returnvalue_2 0)
  (`KismetArrayLibrary.Array_Clear` (`self.AllComponents`))
  (`/Game/BP_ParameterComponent.Init` _amplitude1 (`self.Material`) "Amplitude1" 2.5 (0.0 0.0 0.0) (2.5 10.0) 1.0 true)
  (`KismetArrayLibrary.Array_Add` (`self.AllComponents`) _amplitude1)
  (`/Game/BP_ParameterComponent.Init` _amplitude2 (`self.Material`) "Amplitude2" 2.5 (0.0 0.0 0.0) (2.5 10.0) 1.0 true)
  (`KismetArrayLibrary.Array_Add` (`self.AllComponents`) _amplitude2)
  (`/Game/BP_ParameterComponent.Init` _frequencyx1 (`self.Material`) "FrequencyX1" 2.5 (0.0 0.0 0.0) (2.5 10.0) 1.0 true)
  (`KismetArrayLibrary.Array_Add` (`self.AllComponents`) _frequencyx1)
  (`/Game/BP_ParameterComponent.Init` _frequencyx2 (`self.Material`) "FrequencyX2" 2.5 (0.0 0.0 0.0) (2.5 10.0) 1.0 true)
  (`KismetArrayLibrary.Array_Add` (`self.AllComponents`) _frequencyx2)
  (`/Game/BP_ParameterComponent.Init` _frequencyy1 (`self.Material`) "FrequencyY1" 2.5 (0.0 0.0 0.0) (2.5 10.0) 1.0 true)
  (`KismetArrayLibrary.Array_Add` (`self.AllComponents`) _frequencyy1)
  (`/Game/BP_ParameterComponent.Init` _frequencyy2 (`self.Material`) "FrequencyY2" 2.5 (0.0 0.0 0.0) (2.5 10.0) 1.0 true)
  (`KismetArrayLibrary.Array_Add` (`self.AllComponents`) _frequencyy2)
  (`/Game/BP_ParameterComponent.Init` _rotation (`self.Material`) "Rotation" 0.25 (0.0 0.0 0.0) (0.25 1.0) 0.1 true)
  (`KismetArrayLibrary.Array_Add` (`self.AllComponents`) _rotation)
  (`/Game/BP_ParameterComponent.Init` (`self.RedChannel`) (`self.Material`) " " 0.5 (1.0 0.0 0.0) (0.0 1.0) 1.0 true)
  (`/Game/BP_ParameterComponent.Init` (`self.BlueChannel`) (`self.Material`) " " 0.5 (0.0 0.0 1.0) (0.0 1.0) 0.1 true)
  (`/Game/BP_ParameterComponent.Init` (`self.GreenChannel`) (`self.Material`) " " 0.5 (0.0 1.0 0.0) (0.0 1.0) 0.1 true)
  (`/Game/BP_ParameterComponent.Init` (`self.Height`) (`self.Material`) "UpHeight" 35.0 (0.0 0.0 0.0) (10.0 200.0) 0.1 false)
  (bind _returnvalue_3 (`MaterialInstanceDynamic.K2_GetVectorParameterValue` (`self.Material`) (`|GetArrayItem` (`self.ColorParamName`))))
  (`KismetArrayLibrary.Array_Set` (`self.ColorParamLinearColor`) 0 _returnvalue_3)
  (bind _returnvalue_4 (`MaterialInstanceDynamic.K2_GetVectorParameterValue` (`self.Material`) (`|GetArrayItem` (`self.ColorParamName`) 1)))
  (`KismetArrayLibrary.Array_Set` (`self.ColorParamLinearColor`) 1 _returnvalue_4)
  (set `self.CurColor` (`|GetArrayItem` (`self.ColorParamName`)))
  ; Ignores code for the small sphere that has no "PlayerSphere" reference
  (`/Engine/EditorBlueprintResources/StandardMacros.IsValid` (`self.OtherSphere`)
    (:`Is Valid`
      (`self.RandomizeValues` (`self.OtherSphere`) 0))))

(event `Key|C`
  (params (Key :type "Key Structure"))
  (bind _redchannel (`self.RedChannel`))
  (bind _output (`|GetArrayItem` (`self.ColorParamLinearColor`) (`self.IndexColor`)))
  (:`Pressed`
    (`/Game/BP_ParameterComponent.CallChange` _redchannel (`self.CurColor`) true 0 _output true)
    (`KismetArrayLibrary.Array_Set` (`self.ColorParamLinearColor`) (`self.IndexColor`) (`/Game/BP_ParameterComponent.AimedValueVector` _redchannel)))
  (:`Released`
    (`/Game/BP_ParameterComponent.CallChange` (`self.RedChannel`) "None" false 0 _output false)))

(event `Key|B`
  (params (Key :type "Key Structure"))
  (bind _bluechannel (`self.BlueChannel`))
  (bind _output (`|GetArrayItem` (`self.ColorParamLinearColor`) (`self.IndexColor`)))
  (:`Pressed`
    (`/Game/BP_ParameterComponent.CallChange` _bluechannel (`self.CurColor`) true 0 _output true)
    (`KismetArrayLibrary.Array_Set` (`self.ColorParamLinearColor`) (`self.IndexColor`) (`/Game/BP_ParameterComponent.AimedValueVector` _bluechannel)))
  (:`Released`
    (`/Game/BP_ParameterComponent.CallChange` (`self.BlueChannel`) "None" false 0 _output false)))

(event `Key|Q`
  (params (Key :type "Key Structure"))
  (:`Pressed`
    (`/Game/BP_ParameterComponent.CallChange` :`self` (`self.Amplitude1`) :`IsPress` true :`ValueInt` 1))
  (:`Released`
    (`/Game/BP_ParameterComponent.CallChange` :`self` (`self.Amplitude1`))))

(event `Key|W`
  (params (Key :type "Key Structure"))
  (:`Pressed`
    (`/Game/BP_ParameterComponent.CallChange` :`self` (`self.FrequencyX1`) :`IsPress` true :`ValueInt` 1))
  (:`Released`
    (`/Game/BP_ParameterComponent.CallChange` :`self` (`self.FrequencyX1`))))

(event `Key|E`
  (params (Key :type "Key Structure"))
  (:`Pressed`
    (`/Game/BP_ParameterComponent.CallChange` :`self` (`self.FrequencyX1`) :`IsPress` true :`ValueInt` -1))
  (:`Released`
    (`/Game/BP_ParameterComponent.CallChange` :`self` (`self.FrequencyX1`))))

(event `Key|R`
  (params (Key :type "Key Structure"))
  (:`Pressed`
    (`/Game/BP_ParameterComponent.CallChange` :`self` (`self.Amplitude1`) :`IsPress` true :`ValueInt` -1))
  (:`Released`
    (`/Game/BP_ParameterComponent.CallChange` :`self` (`self.Amplitude1`))))

(event `Key|T`
  (params (Key :type "Key Structure"))
  (:`Pressed`
    (`/Game/BP_ParameterComponent.CallChange` :`self` (`self.FrequencyY1`) :`IsPress` true :`ValueInt` 1))
  (:`Released`
    (`/Game/BP_ParameterComponent.CallChange` :`self` (`self.FrequencyY1`))))

(event `Key|Y`
  (params (Key :type "Key Structure"))
  (:`Pressed`
    (`/Game/BP_ParameterComponent.CallChange` :`self` (`self.FrequencyY1`) :`IsPress` true :`ValueInt` -1))
  (:`Released`
    (`/Game/BP_ParameterComponent.CallChange` :`self` (`self.FrequencyY1`))))

(event `Key|Z`
  (params (Key :type "Key Structure"))
  (:`Pressed`
    (`/Game/BP_ParameterComponent.CallChange` :`self` (`self.Rotation`) :`IsPress` true))
  (:`Released`
    (`/Game/BP_ParameterComponent.CallChange` :`self` (`self.Rotation`))))

(event `Key|A`
  (params (Key :type "Key Structure"))
  (:`Pressed`
    (`/Game/BP_ParameterComponent.CallChange` :`self` (`self.Amplitude2`) :`IsPress` true :`ValueInt` 1))
  (:`Released`
    (`/Game/BP_ParameterComponent.CallChange` :`self` (`self.Amplitude2`))))

(event `Key|S`
  (params (Key :type "Key Structure"))
  (:`Pressed`
    (`/Game/BP_ParameterComponent.CallChange` :`self` (`self.FrequencyX2`) :`IsPress` true :`ValueInt` 1))
  (:`Released`
    (`/Game/BP_ParameterComponent.CallChange` :`self` (`self.FrequencyX2`))))

(event `Key|D`
  (params (Key :type "Key Structure"))
  (:`Pressed`
    (`/Game/BP_ParameterComponent.CallChange` :`self` (`self.FrequencyX2`) :`IsPress` true :`ValueInt` -1))
  (:`Released`
    (`/Game/BP_ParameterComponent.CallChange` :`self` (`self.FrequencyX2`))))

(event `Key|F`
  (params (Key :type "Key Structure"))
  (:`Pressed`
    (`/Game/BP_ParameterComponent.CallChange` :`self` (`self.Amplitude2`) :`IsPress` true :`ValueInt` -1))
  (:`Released`
    (`/Game/BP_ParameterComponent.CallChange` :`self` (`self.Amplitude2`))))

(event `Key|G`
  (params (Key :type "Key Structure"))
  (:`Pressed`
    (`/Game/BP_ParameterComponent.CallChange` :`self` (`self.FrequencyY2`) :`IsPress` true :`ValueInt` 1))
  (:`Released`
    (`/Game/BP_ParameterComponent.CallChange` :`self` (`self.FrequencyY2`))))

(event `Key|H`
  (params (Key :type "Key Structure"))
  (:`Pressed`
    (`/Game/BP_ParameterComponent.CallChange` :`self` (`self.FrequencyY2`) :`IsPress` true :`ValueInt` -1))
  (:`Released`
    (`/Game/BP_ParameterComponent.CallChange` :`self` (`self.FrequencyY2`))))

(event `Key|V`
  (params (Key :type "Key Structure"))
  (bind _greenchannel (`self.GreenChannel`))
  (bind _output (`|GetArrayItem` (`self.ColorParamLinearColor`) (`self.IndexColor`)))
  (:`Pressed`
    (`/Game/BP_ParameterComponent.CallChange` _greenchannel (`self.CurColor`) true 0 _output true)
    (`KismetArrayLibrary.Array_Set` (`self.ColorParamLinearColor`) (`self.IndexColor`) (`/Game/BP_ParameterComponent.AimedValueVector` _greenchannel)))
  (:`Released`
    (`/Game/BP_ParameterComponent.CallChange` (`self.GreenChannel`) "None" false 0 _output false)))

(event `Key|X`
  (params (Key :type "Key Structure"))
  (bind _colorparamname (`self.ColorParamName`))
  (bind _output (`|GetArrayItem` (`self.ColorParamLinearColor`) (`self.IndexColor`)))
  (:`Pressed`
    (bind _result (`/Engine/EditorBlueprintResources/StandardMacros.IncrementInt` (`self.IndexColor`))
      (:`  `
        (if (>= _result (`KismetArrayLibrary.Array_Length` _colorparamname))
          (set `self.IndexColor` 0))
        (bind _output_get (set `self.CurColor` (`|GetArrayItem` _colorparamname (`self.IndexColor`))))
        (`/Game/BP_ParameterComponent.CallChange` (`self.RedChannel`) _output_get false 0 _output true)
        (`/Game/BP_ParameterComponent.CallChange` (`self.GreenChannel`) _output_get false 0 _output true)
        (`/Game/BP_ParameterComponent.CallChange` (`self.BlueChannel`) _output_get false 0 _output true)))))

(event `self.ReceiveTick`
  (params (DeltaSeconds :type "Float (single-precision)"))
  (bind _result (`/Game/BP_ParameterComponent.GetFloatValue` (`self.Height`)))
  (`KismetSystemLibrary.PrintString` (`KismetStringLibrary.Conv_DoubleToString` _result) true true (struct :`G` 0.66 :`B` 1.0 :`A` 1.0) 0.5)
  (`self.ProcessExplosion` 0.0)
  (`/Engine/EditorBlueprintResources/StandardMacros.IsValid` (`self.OtherSphere`)
    (:`Is Valid`
      (bind _issimilar (`self.CompareValues` (`self.HudWidget`)))
      (if _issimilar
        (bind _output_get (set `self.ShaderLevel` (`KismetMathLibrary.Clamp` (+ (`self.ShaderLevel`) 1) 0 (`self.GetMaxParameter`))))
        (`self.RandomizeValues` (`self.OtherSphere`) _output_get)
        (`KismetSystemLibrary.PrintString` (`KismetStringLibrary.Concat_StrStr` "=========================================================" "GOING TO LEVEL " (`KismetStringLibrary.Conv_IntToString` _output_get) "=========================================================") true true (struct :`G` 0.66 :`B` 1.0 :`A` 1.0) 5.0)))))

(event `Key|P`
  (params (Key :type "Key Structure"))
  (bind _linearcolor (make `LinearColor` 1.0 0.25))
  (bind _hudwidget (`self.HudWidget`))
  (bind _height (`self.Height`))
  (bind (_clampvalue_x _clampvalue_y) (`KismetMathLibrary.BreakVector2D` (`/Game/BP_ParameterComponent.ClampValue` _height)))
  (:`Pressed`
    (if (`self.IsExplosionTriggered`)
      (set `self.IsExplosionTriggered` false)
      (set `/Game/UI/WB_Level.IsExploding` false (`self.HudWidget`))
      (set `/Game/BP_ParameterComponent.InUse` true (`self.Height`))
      (set `/Game/BP_ParameterComponent.GoUp` -1 (`self.Height`))
      ; Go back to initial color
      (for (_array_element _array_index) (`self.ColorParamName`)
        (if (== _array_element "ColorIn")
          (bind _output (`|GetArrayItem` (`self.ColorsBeforeExplosionTriggered`) _array_index))
          (`/Game/BP_ParameterComponent.CallAimingChange` (`self.RedChannel`) _output _array_element)
          (bind _returnvalue (`MaterialInstanceDynamic.K2_GetVectorParameterValue` (`self.Material`) _array_element))
          (`KismetSystemLibrary.PrintString` (`KismetStringLibrary.Concat_StrStr` "Valeur actuelle : " (`KismetStringLibrary.Conv_ColorToString` _returnvalue) " / " "valeur d'arrivée : " (`KismetStringLibrary.Conv_ColorToString` _output)) true true (struct :`R` 1.0 :`G` 0.207129 :`B` 0.187233 :`A` 1.0) 50.0)
          (else
            (`/Game/BP_ParameterComponent.CallAimingChange` (`self.BlueChannel`) _output _array_element))))
      (else
        (set `self.IsExplosionTriggered` true)
        ;[0.995 0.15 0.15 0.5] TODO
        (bind _result (`/Game/BP_ParameterComponent.GetFloatValue` _height))
        (set `/Game/UI/WB_Level.ExplodingPercent` (/ (- _clampvalue_y _result) (- _clampvalue_y _clampvalue_x)) _hudwidget)
        (set `/Game/UI/WB_Level.Time` 0.0 _hudwidget)
        (set `/Game/UI/WB_Level.IsExploding` true (`self.HudWidget`))
        (if (== _result 10.0)
          ; Set initial color at the begining of the explosion
          (for _array_element_2 (`self.ColorParamName`)
            (bind _returnvalue_2 (`MaterialInstanceDynamic.K2_GetVectorParameterValue` (`self.Material`) _array_element_2))
            (`KismetArrayLibrary.Array_Add` (`self.ColorsBeforeExplosionTriggered`) _returnvalue_2)))
        (set `/Game/BP_ParameterComponent.InUse` true (`self.Height`))
        ; Explosion effects
        (set `/Game/BP_ParameterComponent.GoUp` 1 (`self.Height`))
        (for _array_element_3 (`self.ColorParamName`)
          (if (== _array_element_3 "ColorIn")
            ;; internal color become yellow
            (`/Game/BP_ParameterComponent.CallAimingChange` (`self.RedChannel`) _linearcolor _array_element_3)
            (`/Game/BP_ParameterComponent.CallAimingChange` (`self.GreenChannel`) _linearcolor _array_element_3)
            (else
              ;; external color become orange
              (`/Game/BP_ParameterComponent.CallAimingChange` (`self.BlueChannel`) (make `LinearColor` 1.0 1.0) _array_element_3))))))))

(fn `CompareValues`
  (params (HudWidget :type "/Game/UI/WB_Level Object Reference"))
  (returns (IsSimilar :type Boolean))
  (locals (TrueValues :type Integer) (CheckedValue :type Integer) (WidgetRef :type "/Game/UI/WB_Level Object Reference"))
  (set `local.WidgetRef` HudWidget)
  (`/Engine/EditorBlueprintResources/StandardMacros.IsValid` (`self.OtherSphere`)
    (:`Is Valid`
      (for (_array_element _array_index) (`self.ColorParamName`)
        ; Compare
        (`/Engine/EditorBlueprintResources/StandardMacros.IncrementInt` (`local.CheckedValue`)
          (:`  `
            (bind _output (`|GetArrayItem` (`self.ColorParamLinearColor`) _array_index))
            (bind _output_2 (`|GetArrayItem` (`/Game/Emilie/BP_Ball_EM.ColorParamLinearColor` (`self.OtherSphere`)) _array_index))
            (bind _returnvalue (`KismetMathLibrary.LinearColor_IsNearEqual` _output _output_2))
            (if _returnvalue
              (`/Engine/EditorBlueprintResources/StandardMacros.IncrementInt` (`local.TrueValues`)
                (:`  `
                  _)))
            (bind (_returnvalue_r _returnvalue_g _returnvalue_b) (break `LinearColor` (- _output _output_2)))
            (`/Game/UI/WB_Level.DisplayParameterMatchingScore` (`self.HudWidget`) _returnvalue (- 1.0 (/ (+ (`KismetMathLibrary.Abs` _returnvalue_r) (`KismetMathLibrary.Abs` _returnvalue_g) (`KismetMathLibrary.Abs` _returnvalue_b)) (* 3.0 1.0))) _array_element))))
      (for (_array_element_2 _array_index_2) (`self.AllComponents`)
        (bind _output_3 (`|GetArrayItem` (`/Game/Emilie/BP_Ball_EM.AllComponents` (`self.OtherSphere`)) _array_index_2))
        (bind _results (`/Game/BP_ParameterComponent.GetVectorValue` _output_3))
        (bind _result (`/Game/BP_ParameterComponent.GetFloatValue` _output_3))
        (bind _parameter_name (`/Game/BP_ParameterComponent.Parameter Name` _array_element_2))
        (bind (_result_2 _percentage) (`/Game/BP_ParameterComponent.CallCompare` _array_element_2 _parameter_name _result _results))
        (`/Game/UI/WB_Level.DisplayParameterMatchingScore` (`self.HudWidget`) _result_2 _percentage _parameter_name)
        (`/Engine/EditorBlueprintResources/StandardMacros.IncrementInt` (`local.CheckedValue`)
          (:`  `
            (if _result_2
              (`/Engine/EditorBlueprintResources/StandardMacros.IncrementInt` (`local.TrueValues`))))))
      (`/Game/UI/WB_Level.UpdateHud` (`self.HudWidget`) (`local.TrueValues`) (`local.CheckedValue`))
      (return (== (`local.CheckedValue`) (`local.TrueValues`))))
    (:`Is Not Valid`
      (return false))))

(fn `ProcessExplosion`
  (params (DeltaTime :type "Float (double-precision)"))
  (locals (Height :type "Float (double-precision)") (MatchingColorAmount :type Integer))
  (bind (_clampvalue_x _clampvalue_y) (`KismetMathLibrary.BreakVector2D` (`/Game/BP_ParameterComponent.ClampValue` (`self.Height`))))
  (if (`self.IsExplosionTriggered`)
    (bind _returnvalue (`MaterialInstanceDynamic.K2_GetScalarParameterValue` (`self.Material`) "UpHeight"))
    (set `local.Height` _returnvalue)
    (if (`KismetMathLibrary.NearlyEqual_FloatFloat` (`local.Height`) _clampvalue_y 1.0)
      (`SceneComponent.SetVisibility` (`self.SphereTooDense`) false false)
      (set `/Game/UI/WB_Level.IsExploding` false (`self.HudWidget`)))
    (elif (`KismetArrayLibrary.Array_IsNotEmpty` (`self.ColorsBeforeExplosionTriggered`))
      (for (_array_element _array_index) (`self.ColorParamName`)
        (bind _returnvalue_2 (`MaterialInstanceDynamic.K2_GetVectorParameterValue` (`self.Material`) _array_element))
        (if (`KismetMathLibrary.LinearColor_IsNearEqual` _returnvalue_2 (`|GetArrayItem` (`self.ColorsBeforeExplosionTriggered`) _array_index) 0.1)
          (`/Engine/EditorBlueprintResources/StandardMacros.IncrementInt` (`local.MatchingColorAmount`))))
      (if (== (`local.MatchingColorAmount`) (`KismetArrayLibrary.Array_Length` (`self.ColorParamName`)))
        (set `/Game/BP_ParameterComponent.InUse` true (`self.Height`))
        (`KismetArrayLibrary.Array_Clear` (`self.ColorsBeforeExplosionTriggered`))))))

(fn `RandomizeValues`
  (params (ShaderLevel :type Integer))
  (bind _bluechannel (`self.BlueChannel`))
  (bind _redchannel (`self.RedChannel`))
  (bind _returnvalue (`KismetArrayLibrary.Array_Length` (`self.ColorParamName`)))
  (bind _output (`|GetArrayItem` (`self.ColorParamName`) 1))
  (bind _output_2 (`|GetArrayItem` (`self.ColorParamName`)))
  (bind _aimedvaluevector (`/Game/BP_ParameterComponent.AimedValueVector` _redchannel))
  (bind _aimedvaluevector_2 (`/Game/BP_ParameterComponent.AimedValueVector` _bluechannel))
  (set `self.ShaderLevel` ShaderLevel)
  (`/Game/BP_ParameterComponent.CallRandomize` _redchannel _output_2)
  (`KismetArrayLibrary.Array_Set` (`self.ColorParamLinearColor`) 0 _aimedvaluevector)
  (`/Game/BP_ParameterComponent.CallChange` (`self.RedChannel`) _output_2 false 0 _aimedvaluevector true)
  (`/Game/BP_ParameterComponent.CallChange` (`self.GreenChannel`) _output_2 false 0 _aimedvaluevector true)
  (if (<= 1 (`self.ShaderLevel`))
    (`/Game/BP_ParameterComponent.CallRandomize` _bluechannel _output)
    (`KismetArrayLibrary.Array_Set` (`self.ColorParamLinearColor`) 1 _aimedvaluevector_2)
    (`/Game/BP_ParameterComponent.CallChange` (`self.BlueChannel`) _output false 0 _aimedvaluevector_2 true)
    (if (>= (`self.ShaderLevel`) _returnvalue)
      (for (_array_element _array_index) (`self.AllComponents`)
        (if (<= _array_index (- (`self.ShaderLevel`) _returnvalue))
          (`/Game/BP_ParameterComponent.CallRandomize` _array_element (`/Game/BP_ParameterComponent.Parameter Name` _array_element)))))))

(fn `UserConstructionScript`)